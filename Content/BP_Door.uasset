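; BP_Door is a locked door that a player opens by interacting while carrying a required item.
; Box overlap toggles a widget's visibility for actors identified as the player through a message call.
; Interacting searches the player's inventory: a match optionally updates the mission and destroys the door, otherwise a popup names the missing item.
; The node that would remove the item from inventory is disconnected, so it is never consumed.
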(event `self.Box.OnComponentBeginOverlap`
  (params (OverlappedComponent :type "PrimitiveComponent Object Reference") (OtherActor :type "Actor Object Reference") (OtherComp :type "PrimitiveComponent Object Reference") (OtherBodyIndex :type Integer) (bFromSweep :type Boolean) (SweepResult :type "HitResult Structure (by ref)"))
  (bind _isplayer (message `/Game/BPI_Player.IsPlayer` OtherActor))
  (if _isplayer
    (`SceneComponent.SetVisibility` (`self.Widget`) true false)))

(event `self.Box.OnComponentEndOverlap`
  (params (OverlappedComponent :type "PrimitiveComponent Object Reference") (OtherActor :type "Actor Object Reference") (OtherComp :type "PrimitiveComponent Object Reference") (OtherBodyIndex :type Integer))
  (bind _isplayer (message `/Game/BPI_Player.IsPlayer` OtherActor))
  (if _isplayer
    (`SceneComponent.SetVisibility` (`self.Widget`) false false)))

(event `/Game/BPI_Interactable.Interacted`
  (params (player :type "/Game/ThirdPerson/Blueprints/BP_ThirdPersonCharacter Object Reference"))
  (for (_array_element _array_index) (`/Game/Inventory/BPC_Inventory.Inventory ` (`/Game/ThirdPerson/Blueprints/BP_ThirdPersonCharacter.BPC_Inventory` player))
    (if (`KismetStringLibrary.EqualEqual_StrStr` _array_element (`self.requiredItem`))
      (set `self.gotRequiredItem` true)
      (break)))
  (if (`self.gotRequiredItem`)
    (if (`self.affectsMission`)
      (`/Game/ThirdPerson/Blueprints/BP_ThirdPersonCharacter.UpdateMission` player (`self.newMission`)))
    (`self.K2_DestroyActor`)
    (else
      (`/Game/ThirdPerson/Blueprints/BP_ThirdPersonCharacter.PopupText` player (`KismetStringLibrary.Concat_StrStr` "Missing item:  " (`self.requiredItem`))))))

(fn `UserConstructionScript`)