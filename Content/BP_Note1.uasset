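; BP_Note1 is a readable note the player can interact with, which can also advance the mission.
; Interacting toggles a WBP_Notes widget filled with the note's text, and on the first interaction updates the player's mission if the note affects it.
; A sphere overlap shows a widget component while the player is near and hides it on exit, also closing the note if it is open.
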(event `/Game/BPI_Interactable.Interacted`
  (params (player :type "/Game/ThirdPerson/Blueprints/BP_ThirdPersonCharacter Object Reference"))
  (if (`self.affectsMission`)
    (`/Game/ThirdPerson/Blueprints/BP_ThirdPersonCharacter.UpdateMission` player (`self.newMission`))
    (set `self.affectsMission` false))
  (`self.TogglePickup`))

(event `TogglePickup`
  (if (`self.isReading`)
    (`self.PutDownNote`)
    (else
      (`self.PickupNote`))))

(event `PickupNote`
  (bind _returnvalue (`|CreateWidget` "/Game/WBP_Notes1.WBP_Notes_C"))
  (set `TextBlock.Text` (`KismetTextLibrary.Conv_StringToText` (`self.noteText`)) (`/Game/WBP_Notes1.TextBlock` _returnvalue))
  (`UserWidget.AddToViewport` _returnvalue 0)
  (set `self.isReading` true))

(event `PutDownNote`
  (`Widget.RemoveFromParent` (stale `PickupNote` _returnvalue))
  (set `self.isReading` false))

(event `self.Sphere.OnComponentBeginOverlap`
  (params (OverlappedComponent :type "PrimitiveComponent Object Reference") (OtherActor :type "Actor Object Reference") (OtherComp :type "PrimitiveComponent Object Reference") (OtherBodyIndex :type Integer) (bFromSweep :type Boolean) (SweepResult :type "HitResult Structure (by ref)"))
  (bind _isplayer (message `/Game/BPI_Player.IsPlayer` OtherActor))
  (if _isplayer
    (`SceneComponent.SetVisibility` (`self.Widget`) true false)))

(event `self.Sphere.OnComponentEndOverlap`
  (params (OverlappedComponent :type "PrimitiveComponent Object Reference") (OtherActor :type "Actor Object Reference") (OtherComp :type "PrimitiveComponent Object Reference") (OtherBodyIndex :type Integer))
  (bind _isplayer (message `/Game/BPI_Player.IsPlayer` OtherActor))
  (if _isplayer
    (`SceneComponent.SetVisibility` (`self.Widget`) false false)
    (if (`self.isReading`)
      (`self.PutDownNote`))))

(fn `UserConstructionScript`)