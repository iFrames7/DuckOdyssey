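; BP_ItemInteract is an interactable item actor that can update the player's mission and is removed once used.
; Its Sphere overlap events show and hide a prompt Widget, using an IsPlayer message on the other actor to respond only to players.
; The Interacted event passes NewMission to the player's UpdateMission when AffectsMission is set, then destroys the actor in either case.
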(event `self.Sphere.OnComponentBeginOverlap`
  (params (OverlappedComponent :type "PrimitiveComponent Object Reference") (OtherActor :type "Actor Object Reference") (OtherComp :type "PrimitiveComponent Object Reference") (OtherBodyIndex :type Integer) (bFromSweep :type Boolean) (SweepResult :type "HitResult Structure (by ref)"))
  (bind _isplayer (message `/Game/BPI_Player.IsPlayer` OtherActor))
  (if _isplayer
    (`SceneComponent.SetVisibility` (`self.Widget`) true false)))

(event `self.Sphere.OnComponentEndOverlap`
  (params (OverlappedComponent :type "PrimitiveComponent Object Reference") (OtherActor :type "Actor Object Reference") (OtherComp :type "PrimitiveComponent Object Reference") (OtherBodyIndex :type Integer))
  (bind _isplayer (message `/Game/BPI_Player.IsPlayer` OtherActor))
  (if _isplayer
    (`SceneComponent.SetVisibility` (`self.Widget`) false false)))

(event `/Game/BPI_Interactable.Interacted`
  (params (player :type "/Game/ThirdPerson/Blueprints/BP_ThirdPersonCharacter Object Reference"))
  (if (`self.affectsMission`)
    (`/Game/ThirdPerson/Blueprints/BP_ThirdPersonCharacter.UpdateMission` player (`self.newMission`)))
  (`self.K2_DestroyActor`))

(fn `UserConstructionScript`)